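; Lobby game mode for local multiplayer character selection, launching the arena when ready.
; On BeginPlay it creates a player and possessed input-receiver pawn per PlayerStart, indexed by numeric tag, and shows the selection menu.
; SpawnPlayer possesses a skin-preview pawn at the receiver's transform, while SpawnPlayerWidget links a menu entry to the receiver.
; PlayerReady sets a Ready flag and opens Green_Arena_Bigger once all stored flags are true.
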(event EventBeginPlay
  (CallFunction|GetPlayerStarts)
  (CallFunction|SpawnInputReceiver)
  (bind _returnvalue (UserInterface|CreateWidget "/Game/Levels/lobby/UI/WBP_char_selec_menu.WBP_char_selec_menu_C"))
  (bind _output_get (Variables|Default|SetmenuWidget _returnvalue))
  (UserInterface|Viewport|AddtoViewport _output_get 0))

(event EventPlayerReady
  (params (char%20index :type Integer))
  (Development|PrintText (Utilities|Text|FormatText "{nb} ready" char%20index))
  (Utilities|Array|SetArrayElem (Variables|Default|Getready) char%20index true)
  (if (CallFunction|IsAllTrue (Variables|Default|Getready))
    (CallFunction|LaunchGame)))

(event EventSpawnPlayer
  (params (character%20index :type Integer) (input%20receiver :type Bp%20Pawn%20Player%20Selec%20Object%20Reference))
  (bind _returnvalue (Game|SpawnActorfromClass "/Game/Levels/lobby/bp_player_show_skin.bp_player_show_skin_C" (Transformation|GetActorTransform input%20receiver) "Undefined" 0 character%20index 0))
  (Pawn|Possess (Game|GetPlayerController character%20index) _returnvalue))

(event EventSpawnPlayerWidget
  (params (character%20index :type Integer))
  (bind _charac_selec_widget (Default|AddCharacSelec (Variables|Default|GetmenuWidget) character%20index))
  (Variables|/Game/Levels/lobby/bp_pawn_player_selec.bp_pawn_player_selec_C|SetCharac%20Select%20Ref (Utilities|Array|Get(acopy) (Variables|Default|Getplayer%20input%20receiver%20array) character%20index) _charac_selec_widget))

(fn ConstructionScript)

(fn GetPlayerStarts
  (bind _outactors (Actor|GetAllActorsOfClass "/Script/Engine.PlayerStart"))
  (Variables|Default|Setplayer%20start%20array _outactors))

(fn SpawnInputReceiver
  (for (_ _array_index) (Variables|Default|Getplayer%20start%20array)
    (LocalVariables|Setindex _array_index)
    (for _array_element (Variables|Default|Getplayer%20start%20array)
      (if (== (CallFunction|NametoInt _array_element) (LocalVariables|Getindex))
        (Class|GameplayStatics|CreatePlayer (LocalVariables|Getindex))
        (bind _returnvalue (Game|SpawnActorfromClass "/Game/Levels/lobby/bp_pawn_player_selec.bp_pawn_player_selec_C" (Transformation|GetActorTransform _array_element) "Undefined" 0 (LocalVariables|Getindex) 0))
        (Utilities|Array|AddUnique (Variables|Default|Getplayer%20input%20receiver%20array) _returnvalue)
        (Utilities|Array|AddUnique (Variables|Default|Getready) false)
        (Pawn|Possess (Game|GetPlayerController (LocalVariables|Getindex)) _returnvalue)
        (Utilities|Array|AddUnique (Variables|Default|Getplayer%20controler%20array) (Game|GetPlayerController (LocalVariables|Getindex)))))))

(fn NametoInt
  (params (name :type Player%20Start%20Object%20Reference))
  (return (Math|Conversions|ToInteger(Byte) (Utilities|String|ToString(Name) (Variables|/Script/Engine.PlayerStart|GetPlayerStartTag name)))))

(fn IsAllTrue
  (params (arr :type Array%20of%20Booleans))
  (bind _array_element (Utilities|Array|ForEachLoopwithBreak arr :!label _label)
    (:LoopBody
      (if (not _array_element)
        (LocalVariables|SetallTrue false)
        (goto _label Break)))
    (:Completed
      (return (LocalVariables|GetallTrue)))))

(fn LaunchGame
  (bind _player_controler_array (Variables|Default|Getplayer%20controler%20array))
  (Development|PrintText (Utilities|Text|FormatText "controller len {nb}" (Utilities|Array|Length _player_controler_array)))
  (for _array_element _player_controler_array
    _)
  (Game|OpenLevel(byObjectReference) "/Game/Levels/Arena/Green_Arena_Bigger.Green_Arena_Bigger"))