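; Lobby actor that displays the selected skin of the player identified by its character index.
; On BeginPlay it reads that player's skin from the game instance and applies the matching Blue or Black material to the skeletal mesh.
; Enter or the gamepad bottom face button sends a player-ready message with the index to the game mode, while B only prints a debug greeting.
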(event EventBeginPlay
  (bind _asgame_instance_bp (Utilities|Casting|CastToGame_instance_BP (Game|GetGameInstance)))
  (bind _player_skin (Default|GetPlayerSkin _asgame_instance_bp (Variables|Default|GetcharIndex)))
  (switch Utilities|FlowControl|Switch|SwitchonSkins _player_skin
    (:NewEnumerator0
      (Development|PrintString "hello 1")
      (Rendering|Material|SetMaterial (Variables|Default|GetSkeletalMesh) 0 "/Game/ImportPack/BattleWizardPolyart/Materials/DefaultSkin.DefaultSkin"))
    (:NewEnumerator1
      (Development|PrintString "Hello 2")
      (Rendering|Material|SetMaterial (Variables|Default|GetSkeletalMesh) 0 "/Game/ImportPack/BattleWizardPolyart/Materials/MaskTintPolyartMatInst02.MaskTintPolyartMatInst02"))))

(event Collision|EventActorBeginOverlap
  (params (OtherActor :type Actor%20Object%20Reference)))

(event EventTick
  (params (DeltaSeconds :type Float%20%28single-precision%29)))

(event Input|KeyboardEvents|B
  (params (Key :type Key%20Structure :default "None"))
  (:Pressed
    (Development|PrintString (Utilities|String|ToString(Text) (Utilities|Text|FormatText "hello from {nb}" (Variables|Default|GetcharIndex))))))

(event Input|KeyboardEvents|Enter
  (params (Key :type Key%20Structure :default "None"))
  (:Pressed
    (Class|BPIGmSelecPlayer|PlayerReady(Message) (Game|GetGameMode) (Variables|Default|GetcharIndex))))

(event Input|GamepadEvents|GamepadFaceButtonBottom
  (params (Key :type Key%20Structure :default "None"))
  (:Pressed
    (Class|BPIGmSelecPlayer|PlayerReady(Message) (Game|GetGameMode) (Variables|Default|GetcharIndex))))

(fn ConstructionScript)