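; Game instance Blueprint that holds match state for a two-player, round-based game.
; It stores each player's skin, score and spells, exposed through setters and getters that select the player by index 0 or 1.
; A round counter can be incremented, and ResetScores zeroes both scores and returns the round to 1.
; GetWinner compares scores and returns a result string, with ties reported as a Player 2 win.
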(fn SetPlayerSkin
  (params (A :type Integer) (PLayer%20Skin :type Skins%20Enum :default "NewEnumerator0"))
  (switch int A
    (:0
      (Variables|Default|SetPLayer%201%20Skin PLayer%20Skin))
    (:1
      (Variables|Default|SetPlayer%202%20skin PLayer%20Skin))))

(fn GetPlayerSkin
  (params (player%20index :type Integer))
  (switch int player%20index
    (:0
      (return (Variables|Default|GetPLayer%201%20Skin)))
    (:1
      (return (Variables|Default|GetPlayer%202%20skin)))))

(fn SetPlayerScore
  (params (Player_index :type Integer) (Player_score :type Integer))
  (switch int Player_index
    (:0
      (Variables|Default|SetPlayer%201%20Score Player_score))
    (:1
      (Variables|Default|SetPlayer%202%20Score Player_score))))

(fn GetPlayerScore
  (params (Player_index :type Integer))
  (switch int Player_index
    (:0
      (return (Variables|Default|GetPlayer%201%20Score)))
    (:1
      (return (Variables|Default|GetPlayer%202%20Score)))))

(fn IncreaseRoundNumber
  (Variables|Default|SetRound%20Number (+ (Variables|Default|GetRound%20Number) 1)))

(fn GetRoundNumber
  (return (Variables|Default|GetRound%20Number)))

(fn GetWinner
  (if (> (Variables|Default|GetPlayer%201%20Score) (Variables|Default|GetPlayer%202%20Score))
    (return "Player 1 win")
    (else
      (return "Player 2 win"))))

(fn ResetScores
  (Variables|Default|SetPlayer%202%20Score 0)
  (Variables|Default|SetPlayer%201%20Score 0)
  (Variables|Default|SetRound%20Number 1))

(fn GetPlayerSpells
  (params (GetPlayerIndex :type Integer))
  (if (== GetPlayerIndex 0)
    (return (Variables|Default|GetPlayer%201%20spells))
    (else
      (return (Variables|Default|GetPlayer%202%20spells)))))

(fn SetPlayerSpells
  (params (PlayerIndex :type Integer) (Spells :type Array%20of%20Strings))
  (if (== PlayerIndex 0)
    (Variables|Default|SetPlayer%201%20spells Spells)
    (else
      (Variables|Default|SetPlayer%202%20spells Spells))))