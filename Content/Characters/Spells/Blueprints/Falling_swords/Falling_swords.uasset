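; Falling swords spell actor, a short-lived area effect that periodically applies damage to wizards inside its sphere and destroys itself after a fixed lifespan.
; Tick drives two independent timers: one spawns Niagara effects at random horizontal offsets around the actor.
; The other applies a negative base damage value to each overlapping BP_Wizard except the spell's owner, who is also passed as damage causer.
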(event EventBeginPlay
  (Actor|SetLifeSpan 3.0))

(event EventTick
  (params (DeltaSeconds :type Float%20%28single-precision%29))
  (Variables|damage|SettickCd (+ (Variables|damage|GettickCd) DeltaSeconds))
  (Variables|swordanim|Setanim%20CD (+ (Variables|swordanim|Getanim%20CD) DeltaSeconds))
  (Utilities|FlowControl|Sequence
    (:then_0
      ;[1 1 1] anim logic
      (if (>= (Variables|swordanim|Getanim%20CD) (Variables|swordanim|Getanim%20delay))
        (Variables|swordanim|Setanim%20CD 0.0)
        (AddComponent|AddNiagaraComponent false (Math|Transform|MakeTransform (Math|Vector|MakeVector (Math|Random|RandomFloatinRange -2e+02 2e+02) (Math|Random|RandomFloatinRange -2e+02 2e+02) 0.0) "0, 0, 0" "1.000000,1.000000,1.000000"))))
    (:then_1
      ;[1 1 1] damage logic
      (if (>= (Variables|damage|GettickCd) (Variables|Damage|GettickDelay))
        (Variables|damage|SettickCd 0.0)
        (for _array_element (Collision|GetOverlappingActors (Variables|Default|GetSphere) "/Game/Characters/BP_Wizard.BP_Wizard_C" :!class /Script/Engine.PrimitiveComponent)
          (if (!= _array_element (Components|GetOwner))
            (Game|Damage|ApplyDamage _array_element -2.0 0 (Components|GetOwner))))))))

(fn ConstructionScript)