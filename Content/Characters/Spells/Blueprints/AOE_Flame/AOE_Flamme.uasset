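; AOE_Flamme is a short-lived area-of-effect flame spell actor that applies damage once, shortly after it spawns.
; One tick after BeginPlay, it applies damage with a negative base value to every actor overlapping its Sphere except its owner, printing a debug string per hit.
; It then plays the Explosion effect for about a second, and its life span removes it just afterwards.
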(event EventBeginPlay
  (Actor|SetLifeSpan 1.1)
  (Utilities|FlowControl|DelayUntilNextTick)
  (CallFunction|DealDamage)
  ;[1 1 1] animation
  (Components|Activation|Activate (Variables|Default|Getexplosion) false)
  (Utilities|FlowControl|Delay 1.0)
  (Components|Activation|Deactivate (Variables|Default|Getexplosion)))

(fn ConstructionScript)

(fn DealDamage
  (bind _returnvalue (Components|GetOwner))
  (for _array_element (Collision|GetOverlappingActors (Variables|Collision|GetSphere) 0 :!class /Script/Engine.PrimitiveComponent)
    (if (!= _array_element _returnvalue)
      (Game|Damage|ApplyDamage _array_element -5e+01 0 _returnvalue)
      (Development|PrintString "Hello"))))