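; Burn status effect that deals damage over time to an afflicted player until it expires.
; UpdateTick accumulates delta time toward a tick delay, then resets it and applies damage to the player, crediting the status dealer as the damage causer.
; The same update counts down the duration and, once it runs out, has the effect remove itself from the owning status component.
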(fn UpdateTick
  (params (Affected%20Player :type BP%20Wizard%20Object%20Reference) (deltaTime :type Float%20%28double-precision%29) (status%20component :type Status%20Component%20Object%20Reference))
  ;[1 1 1] update tick cooldown
  (Variables|Default|SettickCD (+ (Variables|Default|GettickCD) deltaTime))
  ;[1 1 1] decrease duration
  (Variables|Default|Setduration (- (Variables|Default|Getduration) deltaTime))
  (Utilities|FlowControl|Sequence
    (:then_0
      ;[1 1 1] main logic
      ;;[1 1 1] check if tick delay is done
      (if (>= (Variables|Default|GettickCD) (Variables|Default|GettickDelay))
        ;;[1 1 1] reset tick CD
        (Variables|Default|SettickCD 0.0)
        ;;[1 1 1] damage dealing
        (Game|Damage|ApplyDamage Affected%20Player (Variables|Default|Getdmg) 0 (Variables|Default|GetStatus%20Dealer))))
    (:then_1
      ;[1 1 1] remove itself when duration expire
      (if (<= (Variables|Default|Getduration) 0.0)
        (CallFunction|RemoveSelf status%20component)))))