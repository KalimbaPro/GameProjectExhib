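; Player character Blueprint with temporary hard-coded controls for turning the view and applying damage.
; Z/S and Q/D key presses add fixed controller pitch and yaw steps, once per press rather than continuously.
; Left mouse click calls ApplyAnyDamage on the DamageComponent with the first player controller as instigator.
; BeginPlay, overlap, Tick and the construction script are empty.
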(event EventBeginPlay)

(event Collision|EventActorBeginOverlap
  (params (OtherActor :type Actor%20Object%20Reference)))

(event EventTick
  (params (DeltaSeconds :type Float%20%28single-precision%29)))

(event Input|MouseEvents|LeftMouseButton
  (params (Key :type Key%20Structure))
  (:Pressed
    (Default|ApplyAnyDamage (Variables|Default|GetDamageComponent) 0 (Game|GetPlayerController 0))))

(event Input|KeyboardEvents|Z
  (params (Key :type Key%20Structure))
  ;[0 0 0] Tempo Movement Inputs
  ;;[0.05098 0.05098 0.05098 1 14] Up
  (:Pressed
    (Pawn|Input|AddControllerPitchInput 1.0)))

(event Input|KeyboardEvents|S
  (params (Key :type Key%20Structure))
  ;[0 0 0] Tempo Movement Inputs
  ;;[0.05098 0.05098 0.05098 1 14] Down
  (:Pressed
    (Pawn|Input|AddControllerPitchInput -1.0)))

(event Input|KeyboardEvents|D
  (params (Key :type Key%20Structure))
  ;[0 0 0] Tempo Movement Inputs
  ;;[0.05098 0.05098 0.05098 1 14] Right
  (:Pressed
    (Pawn|Input|AddControllerYawInput 1.0)))

(event Input|KeyboardEvents|Q
  (params (Key :type Key%20Structure))
  ;[0 0 0] Tempo Movement Inputs
  ;;[0.05098 0.05098 0.05098 1 14] Left
  (:Pressed
    (Pawn|Input|AddControllerYawInput -1.0)))

(fn ConstructionScript)